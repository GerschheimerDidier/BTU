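; BTU_GI, likely the Game Instance, manages multiplayer sessions through host, join and leave events.
; Hosting creates a four-slot non-LAN session and opens MainLevel as a listen server.
; Joining searches for sessions and calls JoinSession on every result without stopping at the first.
; Leaving destroys the session and returns to MainMenu even on failure, with all outcomes except successful hosting reported through debug prints.
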(event Custom|GI_HostGame
  (params (Host :type BTU%20PC%20Object%20Reference))
  (|Session Host 4 false
    (:OnSuccess
      (Game|OpenLevel(byName) "MainLevel" true "listen"))
    (:OnFailure
      (Development|PrintString "Could not create session" true true "(R=0.500000,G=0.000000,B=0.000000,A=1.000000)"))))

(event Custom|GJ_LeaveGame
  (params (NewParam :type BTU%20PC%20Object%20Reference))
  (|DestroySession NewParam
    (:OnSuccess
      (Development|PrintString "Session Destroyed" true true "(R=0.000000,G=0.498039,B=0.000000,A=1.000000)"))
    (:OnFailure
      (Development|PrintString "Could not destroy session" true true "(R=0.500000,G=0.000000,B=0.000000,A=1.000000)")))
  (Game|OpenLevel(byName) "MainMenu"))

(event Custom|GJ_JoinGame
  (params (PC :type BTU%20PC%20Object%20Reference))
  (bind _results (|FindSessions PC 5 false)
    (:OnSuccess
      (for _array_element _results
        (|JoinSession PC _array_element
          (:OnSuccess
            (Development|PrintString "Joining session" true true "(R=0.000000,G=0.498039,B=0.000000,A=1.000000)"))
          (:OnFailure
            (Development|PrintString "Could not join session" true true "(R=0.500000,G=0.000000,B=0.000000,A=1.000000)")))))
    (:OnFailure
      (Development|PrintString "Could not find session" true true "(R=0.500000,G=0.000000,B=0.000000,A=1.000000)"))))