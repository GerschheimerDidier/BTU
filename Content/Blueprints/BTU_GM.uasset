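; BTU_GM is a game mode Blueprint that spawns a Bomb at the origin on BeginPlay and controls round start and end.
; A start request is guarded by GameOn, then prints a timed Ready, Set, Go countdown.
; Start and end notify every actor implementing the Startable interface.
; SelectSpawnPoint returns the first PlayerStart not tagged Taken and tags it to reserve it.
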(event Custom|EndGame
  (Variables|Default|SetGameOn false)
  (bind _outactors (Actor|GetAllActorswithInterface "/Game/Blueprints/Startable.Startable_C"))
  (for _array_element _outactors
    (Class|Startable|OnGameEnd(Message) _array_element)))

(event Custom|StartGame
  (Development|PrintString "Ready")
  (Utilities|FlowControl|Delay 1.5)
  (Development|PrintString "Set")
  (Utilities|FlowControl|Delay 1.5)
  (Development|PrintString "Go!")
  (bind _outactors (Actor|GetAllActorswithInterface "/Game/Blueprints/Startable.Startable_C"))
  (for _array_element _outactors
    (Class|Startable|OnGameStart(Message) _array_element)))

(event Custom|Req_StartGame
  (if (not (Variables|Default|GetGameOn))
    (Variables|Default|SetGameOn true)
    (CallFunction|StartGame)))

(event EventBeginPlay
  (bind _returnvalue (Game|SpawnActorfromClass "/Game/Blueprints/Bomb.Bomb_C" (Math|Transform|MakeTransform "0, 0, 0") "AlwaysSpawn" 0 0))
  (Variables|Default|SetBombRef _returnvalue))

(fn ConstructionScript)

(fn SelectSpawnPoint
  (bind _outactors (Actor|GetAllActorsOfClass "/Script/Engine.PlayerStart"))
  (for _array_element _outactors
    (if (not (Actor|ActorHasTag _array_element "Taken"))
      (Variables|/Script/Engine.Actor|SetTags _array_element (Utilities|Array|MakeArray "Taken"))
      (return _array_element)))
  (return 0))