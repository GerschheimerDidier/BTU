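; BTU_PC is a player controller that passes session host, join and leave requests to the BTU_GI game instance.
; Its Player_Server host and join events, plus the Exit input action, each cast the game instance and call the matching function with the controller itself.
; On BeginPlay with authority it calls CreateHUD, which is an empty event here.
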(event Custom|CreateHUD)

(event Custom|Player_Server_HostGame
  (bind _asbtu_gi (Utilities|Casting|CastToBTU_GI (Game|GetGameInstance)))
  (Default|GIHostGame _asbtu_gi self))

(event Custom|Player_Server_JoinGame
  (bind _asbtu_gi (Utilities|Casting|CastToBTU_GI (Game|GetGameInstance)))
  (Default|GJJoinGame _asbtu_gi self))

(event EventBeginPlay
  (Networking|SwitchHasAuthority
    (:Authority
      (CallFunction|CreateHUD))))

(event Input|ActionEvents|InputActionExit
  (params (Key :type Key%20Structure))
  (:Pressed
    (bind _asbtu_gi (Utilities|Casting|CastToBTU_GI (Game|GetGameInstance)))
    (Default|GJLeaveGame _asbtu_gi self)))

(fn ConstructionScript)