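; Player character for a bomb-passing game, with movement along actor yaw that stays gated until game start.
; Passing the bomb away sets a brief timed insensibility window.
; Death applies damage to a Destructible, disables movement, blends the view to an EndGameCam and hides the mesh on a timer.
; Debug leftovers include a left-trigger kill and printing of stored input axis values.
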(event Custom|OnPlayerKill
  (CallFunction|KillPlayer)
  (bind _returnvalue (Utilities|Time|SetTimerbyEvent (delegate Custom|HideBody) 2.0)))

(event Custom|OnBombPassAway
  (Variables|Default|SetIsInsensible true)
  (bind _returnvalue (Utilities|Time|SetTimerbyEvent (delegate Custom|OnEndInvicibility) 1.5)))

(event Custom|OnEndInvicibility
  (Variables|Default|SetIsInsensible false)
  (Utilities|Time|ClearandInvalidateTimerbyHandle (stale Custom|OnBombPassAway _returnvalue)))

(event Custom|HideBody
  (Rendering|SetVisibility (Variables|Character|GetMesh) false true)
  (Utilities|Time|ClearandInvalidateTimerbyHandle (stale Custom|OnPlayerKill _returnvalue)))

(event EventOnGameStart
  (Variables|Default|SetCanMove true))

(event Input|AxisEvents|InputAxisMove_Forward
  (params (AxisValue :type Float%20%28single-precision%29))
  (bind _output_get (Variables|Default|SetCurrRotationValues (Math|Vector|MakeVector AxisValue (.y (Variables|Default|GetCurrRotationValues)) (.z (Variables|Default|GetCurrRotationValues)))))
  (Development|PrintString (Utilities|String|ToString(Vector) _output_get))
  (if (Variables|Default|GetCanMove)
    (Pawn|Input|AddMovementInput (Math|Vector|GetForwardVector (Math|Rotator|MakeRotator 0.0 0.0 (.yaw (Transformation|GetActorRotation)))) AxisValue false)))

(event Input|AxisEvents|InputAxisMoveRIGHT
  (params (AxisValue :type Float%20%28single-precision%29))
  (Variables|Default|SetCurrRotationValues (Math|Vector|MakeVector (.x (Variables|Default|GetCurrRotationValues)) AxisValue (.z (Variables|Default|GetCurrRotationValues))))
  (if (Variables|Default|GetCanMove)
    (Pawn|Input|AddMovementInput (Math|Vector|GetRightVector (Math|Rotator|MakeRotator 0.0 0.0 (.yaw (Transformation|GetActorRotation)))) AxisValue false)))

(event Input|GamepadEvents|GamepadLeftTrigger
  (params (Key :type Key%20Structure))
  ;[1 0.6231 0] DEBUG
  (:Pressed
    (CallFunction|KillPlayer)
    (bind _returnvalue (Utilities|Time|SetTimerbyEvent (delegate Custom|HideBody) 2.0))))

(fn ConstructionScript)

(fn KillPlayer
  (Class|DestructibleComponent|ApplyDamage (Variables|Default|GetDestructible) 999.0 (Transformation|GetActorLocation) (Math|Vector|GetForwardVector (Transformation|GetWorldRotation (Variables|Character|GetMesh))) 5e+01)
  (Variables|Default|SetCanMove false)
  (Variables|Default|SetIsAlive false)
  (bind _outactors (Actor|GetAllActorsOfClass "/Game/Blueprints/EndGameCam.EndGameCam_C"))
  (bind _asbtu_pc (Utilities|Casting|CastToBTU_PC (Pawn|GetController)))
  (Game|Player|SetViewTargetwithBlend _asbtu_pc (Utilities|Array|Get(acopy) _outactors) 2.0 "VTBlend_Linear" 0.0 false))