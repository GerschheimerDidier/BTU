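; Hot-potato bomb actor that follows a random player character and kills them when its random timer expires.
; Players pass it through SetNewTarget, which accepts only the current holder handing off to a listed, living, non-insensible player.
; After exploding, it hides, drops the victim from the target list and re-arms on another after a random delay.
; It calls EndGame on BTU_GM when too few players remain.
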(event Custom|Boom
  ;[1 1 1] Bomb mechanics
  (Utilities|Time|ClearandInvalidateTimerbyHandle (Variables|Default|GetTimerHandle))
  (CallFunction|DoBoom))

(event Custom|ServerSetTarget
  (params (NewTarget :type BTU%20Player%20Character%20Object%20Reference))
  (CallFunction|ClientonBombSet NewTarget))

(event Custom|ClientOnBombSet
  (params (NewTarget :type BTU%20Player%20Character%20Object%20Reference))
  (Utilities|IsValid NewTarget
    (:Is%20Valid
      (Rendering|SetVisibility (Variables|Default|GetSphere) true false))
    (:Is%20Not%20Valid
      (Rendering|SetVisibility (Variables|Default|GetSphere) false false))))

(event Custom|Play%20sound
  (Audio|PlaySoundatLocation "/Game/Music/EXPLOSION_8.EXPLOSION_8" (Transformation|GetActorLocation)))

(event Custom|req_play_sound
  (CallFunction|PlaySound))

(event Custom|Do%20Bomb%20things
  ;[1 1 1] Bomb mechanics
  (Utilities|FlowControl|Delay (Math|Random|RandomFloatinRange (Variables|Default|GetMin_BombReactivationDelay) (Variables|Default|GetMax_BombReactivationDelay)))
  (CallFunction|GetRandomVictim)
  (bind _returnvalue (Utilities|Time|SetTimerbyEvent (delegate Custom|Boom) (Math|Random|RandomFloatinRange (Variables|Default|GetMinTimer) (Variables|Default|GetMaxTimer))))
  (Variables|Default|SetTimerHandle _returnvalue))

(event Custom|SetNewTarget
  (params (NewTarget :type BTU%20Player%20Character%20Object%20Reference) (Instigator :type BTU%20Player%20Character%20Object%20Reference))
  ;[1 1 1] Set New Target (call from PlayerCharacter)
  (Utilities|CheckNewTargetValidity NewTarget Instigator
    (:Valid
      (Variables|Default|SetTarget NewTarget)
      (Default|OnBombPassAway Instigator))))

(event Custom|OnPlayerDeath
  (params (NewParam :type BTU%20Player%20Character%20Object%20Reference))
  (Utilities|Array|RemoveItem (Variables|Default|GetTargetList) NewParam)
  (if (<= (Utilities|Array|Length (Variables|Default|GetTargetList)) 1)
    (bind _asbtu_gm (Utilities|Casting|CastToBTU_GM (Game|GetGameMode)))
    (Default|EndGame _asbtu_gm)
    (elif (== NewParam (Variables|Default|GetTarget))
      (CallFunction|ClientonBombSet))))

(event EventTick
  (params (DeltaSeconds :type Float%20%28single-precision%29))
  (bind _target (Variables|Default|GetTarget))
  (Utilities|IsValid _target
    (:Is%20Valid
      (Transformation|SetActorLocation (Transformation|GetActorLocation _target) false false))))

(event EventOnGameStart
  ;[1 1 1] Bomb mechanics
  (CallFunction|SetupPlayerList)
  (if (<= (Utilities|Array|Length (Variables|Default|GetTargetList)) 1)
    (Variables|Default|SetEmptyGame true)
    (else
      (CallFunction|GetRandomVictim)
      (bind _returnvalue (Utilities|Time|SetTimerbyEvent (delegate Custom|Boom) (Math|Random|RandomFloatinRange (Variables|Default|GetMinTimer) (Variables|Default|GetMaxTimer))))
      (Variables|Default|SetTimerHandle _returnvalue))))

(fn ConstructionScript)

(fn DoBoom
  (bind _target (Variables|Default|GetTarget))
  (Utilities|IsValid _target
    (:Is%20Valid
      (Default|OnPlayerKill _target)
      (Rendering|SetVisibility (Variables|Default|GetSphere) false true)
      (Utilities|Array|RemoveItem (Variables|Default|GetTargetList) _target)
      (CallFunction|ReqPlaySound)
      (CallFunction|DoBombThings))))

(fn GetRandomVictim
  (bind _targetlist (Variables|Default|GetTargetList))
  (bind _returnvalue (Utilities|Array|Length _targetlist))
  (Utilities|ShouldEndGame _returnvalue
    (:Yes
      ;[1 1 1] Game End
      (bind _asbtu_gm (Utilities|Casting|CastToBTU_GM (Game|GetGameMode)))
      (Default|EndGame _asbtu_gm))
    (:No
      ;[1 1 1] Get Next Target
      (bind _output_get (Variables|Default|SetTarget (Utilities|Array|Get(acopy) _targetlist (- (Math|Random|RandomIntegerinRange 1 _returnvalue) 1))))
      (Networking|SwitchHasAuthority
        (:Authority
          (CallFunction|ClientonBombSet _output_get))))))

(fn GetVictimList)

(fn SetupPlayerList
  (Utilities|Array|Clear (Variables|Default|GetTargetList))
  (bind _outactors (Actor|GetAllActorsOfClass "/Game/Blueprints/BTU_PlayerCharacter.BTU_PlayerCharacter_C"))
  (for _array_element _outactors
    (Utilities|IsValid _array_element
      (:Is%20Valid
        (Utilities|Array|Add (Variables|Default|GetTargetList) _array_element))))
  (Variables|Default|SetEmptyGame false))